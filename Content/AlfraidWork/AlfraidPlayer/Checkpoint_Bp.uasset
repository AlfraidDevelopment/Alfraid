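; Checkpoint trigger actor that saves the player's location when its box is overlapped.
; On overlap it stores the AlfraidPawn player character's location and prints a debug message.
; It then writes that location into a Checkpoint save object in the "check" slot, loading the existing save or creating one if none exists.
; The overlapping actor is not checked, so any overlap records player zero's position.
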(event OnComponentBeginOverlap(Box)
  (params (OverlappedComponent :type Primitive%20Component%20Object%20Reference) (OtherActor :type Actor%20Object%20Reference) (OtherComp :type Primitive%20Component%20Object%20Reference) (OtherBodyIndex :type Integer) (bFromSweep :type Boolean) (SweepResult :type Hit%20Result%20Structure%20%28by%20ref%29))
  (Utilities|FlowControl|Sequence
    (:then_0
      (bind _asalfraid_pawn (Utilities|Casting|CastToAlfraidPawn (Game|GetPlayerCharacter 0)))
      (Variables|Default|Setplayer_loc (Transformation|GetActorLocation _asalfraid_pawn))
      (Development|PrintString "Checkpoint Reached"))
    (:then_1
      (bind _returnvalue (SaveGame|DoesSaveGameExist "check"))
      (if _returnvalue
        (bind _returnvalue_2 (SaveGame|LoadGamefromSlot "check"))
        (bind _ascheckpoint (Utilities|Casting|CastToCheckpoint _returnvalue_2))
        (Variables|/Game/AlfraidWork/AlfraidPlayer/Checkpoint.Checkpoint_C|Setplayer_loc _ascheckpoint (Variables|Default|Getplayer_loc))
        (SaveGame|SaveGametoSlot _ascheckpoint "check")
        (else
          (bind _returnvalue_3 (SaveGame|CreateSaveGameObject "/Game/AlfraidWork/AlfraidPlayer/Checkpoint.Checkpoint_C"))
          (Variables|/Game/AlfraidWork/AlfraidPlayer/Checkpoint.Checkpoint_C|Setplayer_loc _returnvalue_3 (Variables|Default|Getplayer_loc))
          (SaveGame|SaveGametoSlot _returnvalue_3 "check"))))))

(event EventBeginPlay)

(event Collision|EventActorBeginOverlap
  (params (OtherActor :type Actor%20Object%20Reference)))

(event EventTick
  (params (DeltaSeconds :type Float%20%28single-precision%29)))

(fn ConstructionScript)